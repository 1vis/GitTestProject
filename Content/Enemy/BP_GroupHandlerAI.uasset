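; BP_GroupHandlerAI is a group handler actor that gathers every BP_EnemyCharacter in the level at BeginPlay and gives each its index.
; Each Tick it moves itself along its local X axis by Speed and recomputes a line formation sized to the group around its location and forward vector.
; The resulting positions are stored in DesiredPositions and drawn as debug points; this graph itself does not move the enemies.
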(event `self.ReceiveBeginPlay`
  (bind _outactors (`GameplayStatics.GetAllActorsOfClass` "/Game/Enemy/BP_EnemyCharacter.BP_EnemyCharacter_C"))
  (bind _output_get (set `self.EnemyGroup` _outactors))
  (for (_array_element _array_index) _output_get
    (set `/Game/Enemy/BP_EnemyCharacter.Index` _array_index _array_element)))

(event `self.ReceiveTick`
  (params (DeltaSeconds :type "Float (single-precision)"))
  (`self.K2_AddActorLocalOffset` (`KismetMathLibrary.MakeVector` (* DeltaSeconds (`self.Speed`))))
  (bind _output_get (set `self.DesiredPositions` (`GitFormation.GetLineFormation` (`KismetArrayLibrary.Array_Length` (`self.EnemyGroup`)) 150.0 150.0 (`self.K2_GetActorLocation`) (`self.GetActorForwardVector`))))
  (for _array_element _output_get
    (`KismetSystemLibrary.DrawDebugPoint` _array_element 10.0 (struct :`R` 1.0 :`G` 1.0 :`A` 1.0) 0.0)))

(fn `UserConstructionScript`)