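; BP_EnemyCharacter is an enemy character that moves as a member of a group managed by a BP_GitGroupAgent actor.
; On BeginPlay it registers with the first group agent found in the level.
; Each tick it matches the group's speed when near its assigned member position, otherwise switches to a fixed catch-up walk speed.
; The construction script gives the mesh a random MainColor material tint.
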(event `self.ReceiveBeginPlay`
  (bind _outactors (`GameplayStatics.GetAllActorsOfClass` "/Game/Enemy/BP_GitGroupAgent.BP_GitGroupAgent_C"))
  (bind _output_get (set `self.GroupAgent` (`|GetArrayItem` _outactors)))
  (`GitGroupAgent.AddMember` _output_get self))

(event `self.ReceiveTick`
  (params (DeltaSeconds :type "Float (single-precision)"))
  (if (<= (`KismetMathLibrary.VSize` (- (`self.K2_GetActorLocation`) (`GitGroupAgent.GetMemberPosition` (`self.GroupAgent`) self))) 120.0)
    (`self.SetMaxMovementSpeed` (`/Game/Enemy/BP_GitGroupAgent.Speed` (`self.GroupAgent`)))
    (else
      (`self.SetMaxMovementSpeed` 600.0))))

(fn `SetMaxMovementSpeed`
  (params (NewSpeed :type "Float (double-precision)"))
  (set `CharacterMovementComponent.MaxWalkSpeed` NewSpeed (`self.CharacterMovement`))
  (return))

(fn `UserConstructionScript`
  (`MeshComponent.SetVectorParameterValueOnMaterials` (`self.Mesh`) "MainColor" (`KismetMathLibrary.Conv_LinearColorToVector` (`KismetMathLibrary.MakeColor` (`KismetMathLibrary.RandomFloat`) (`KismetMathLibrary.RandomFloat`) (`KismetMathLibrary.RandomFloat`)))))