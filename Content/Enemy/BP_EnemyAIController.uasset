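; AI controller that keeps an enemy in its assigned slot within a group formation.
; On BeginPlay it caches the first BP_GroupHandlerAI found in the level.
; Every Tick it moves the controlled BP_EnemyCharacter to the handler's desired position for that enemy's index.
; The enemy matches the group's speed when near that position and switches to a fixed catch-up speed when farther away.
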(event `self.ReceiveBeginPlay`
  (bind _outactors (`GameplayStatics.GetAllActorsOfClass` "/Game/Enemy/BP_GroupHandlerAI.BP_GroupHandlerAI_C"))
  (set `self.GroupHandlerRef` (`|GetArrayItem` _outactors)))

(event `self.ReceiveTick`
  (params (DeltaSeconds :type "Float (single-precision)"))
  (bind _enemycharacter (`self.EnemyCharacter`))
  (bind _asbp_enemy_character (cast `/Game/Enemy/BP_EnemyCharacter` (`self.K2_GetPawn`)))
  (bind _output_get (set `self.EnemyCharacter` _asbp_enemy_character))
  (bind _output (`|GetArrayItem` (`/Game/Enemy/BP_GroupHandlerAI.DesiredPositions` (`self.GroupHandlerRef`)) (`/Game/Enemy/BP_EnemyCharacter.Index` _output_get)))
  (set `self.bIsCloseEnough` (<= (`KismetMathLibrary.VSize` (- _output (`self.K2_GetActorLocation` (`self.EnemyCharacter`)))) 75.0))
  (`self.MoveToLocation` _output 50.0)
  (if (`self.bIsCloseEnough`)
    (`/Game/Enemy/BP_EnemyCharacter.SetMaxMovementSpeed` _enemycharacter (`/Game/Enemy/BP_GroupHandlerAI.Speed` (`self.GroupHandlerRef`)))
    (else
      (`/Game/Enemy/BP_EnemyCharacter.SetMaxMovementSpeed` _enemycharacter 600.0))))

(fn `UserConstructionScript`)