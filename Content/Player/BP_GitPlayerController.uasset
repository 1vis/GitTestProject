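; Player controller that handles box selection of player characters and attack orders on enemies.
; On BeginPlay it binds to the CheckTheObjectForAction delegate; when the actor under the cursor is an enemy character, it passes it to SetAttackPoint.
; When the selection box has non-zero width and height, it rebuilds SelectedPawns by testing every BP_PlayerCharacter against the box, then highlights their character panels.
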(event `self.ReceiveBeginPlay`
  (add `self.CheckTheObjectForAction` (delegate `Check for the action`)))

(event `Check for the action` :!signature `self.CheckTheObjectForAction`
  (params (ActorUnderCursor :type "Actor Object Reference"))
  (if (`KismetMathLibrary.ClassIsChildOf` (`GameplayStatics.GetObjectClass` ActorUnderCursor) "/Game/Enemy/BP_EnemyCharacter.BP_EnemyCharacter_C")
    (bind _asbp_enemy_character (cast `/Game/Enemy/BP_EnemyCharacter` ActorUnderCursor))
    (`self.Attack` _asbp_enemy_character)))

(fn `Attack`
  (params (`Enemy target` :type "Pawn Object Reference"))
  (`self.SetAttackPoint` `Enemy target`))

(fn `CheckObjectsInsideSelectBox`
  (if (!= (`self.SelectionBoxW`) 0.0)
    (if (!= (`self.SelectionBoxH`) 0.0)
      (`self.GoCheck`))))

(fn `GoCheck`
  (bind _selectedpawns (`self.SelectedPawns`))
  (`KismetArrayLibrary.Array_Clear` (`self.SelectedPawns`))
  (bind _outactors (`GameplayStatics.GetAllActorsOfClass` "/Game/Player/BP_PlayerCharacter.BP_PlayerCharacter_C"))
  (for _array_element _outactors
    (bind _returnvalue (`self.IsInSelectionBox` _array_element))
    (if _returnvalue
      (`KismetArrayLibrary.Array_Add` _selectedpawns _array_element)))
  (`self.HighlightCharacterPanels` _selectedpawns))

(fn `UserConstructionScript`)