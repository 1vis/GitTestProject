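; Player HUD Blueprint that shows the main UI widget and draws the drag selection box for unit or object selection.
; On BeginPlay it caches BP_GitPlayerController, then creates MainUI and adds it to the viewport; SetVisibilityHUD controls that widget's visibility.
; Each DrawHUD draws a translucent blue rectangle from the controller's selection box values, then has the controller check which objects are inside it.
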(event `self.ReceiveBeginPlay`
  (bind _asbp_git_player_controller (cast `/Game/Player/BP_GitPlayerController` (`GameplayStatics.GetPlayerController` 0)))
  (bind _output_get (set `self.PlayerController` _asbp_git_player_controller))
  (bind _returnvalue (`|CreateWidget` "/Game/UI/MainUI.MainUI_C" _output_get))
  (bind _output_get_2 (set `self.MainGUI` _returnvalue))
  (`UserWidget.AddToViewport` _output_get_2 0))

(event `self.ReceiveDrawHUD`
  (params (SizeX :type Integer) (SizeY :type Integer))
  (`self.DrawSelectionBox`))

(event `SetVisibilityHUD`
  (params (NewParam :type "ESlateVisibility Enum"))
  (`Widget.SetVisibility` (`self.MainGUI`) NewParam))

(fn `DrawSelectionBox`
  (bind _playercontroller (`self.PlayerController`))
  (`self.DrawRect` (struct :`R` 0.035113 :`G` 0.103599 :`B` 0.285 :`A` 0.347) (`GitPlayerController.SelectionBoxX` _playercontroller) (`GitPlayerController.SelectionBoxY` _playercontroller) (`GitPlayerController.SelectionBoxW` _playercontroller) (`GitPlayerController.SelectionBoxH` _playercontroller))
  (`/Game/Player/BP_GitPlayerController.CheckObjectsInsideSelectBox` _playercontroller))

(fn `UserConstructionScript`)