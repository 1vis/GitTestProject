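; Selectable squad character that attacks enemies, picks up items and weapons, and dies when health runs out.
; Tick polls attack and interaction states, using line traces and range checks to chase and fire at targets or interact with items.
; Attacking alerts nearby enemies after a random delay by writing itself to their AI blackboards.
; AddWeapon attaches the weapon and swaps the anim blueprint, while death unpossesses, notifies and destroys the actor.
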(event `/Game/Gameplay/Combat/iDamagableChar.Affect Health`
  (params (`Amount of taken Damage` :type "Float (single-precision)"))
  ;[1 1 1] Affecting the players Health section
  (`self.HandleDamage` `Amount of taken Damage`)
  (`self.CalculateUIHealth`)
  (if (`self.IsDead`)
    _))

(event `self.ReceiveBeginPlay`
  (`|ExecutionSequence`
    (:`then_1`
      (`SceneComponent.SetVisibility` (`self.Selection ring decal`) false false)
      (bind _outactors (`GameplayStatics.GetAllActorsOfClass` "/Game/Player/BP_Camera.BP_Camera_C"))
      (`self.SetOwner` (`|GetArrayItem` _outactors))
      (set `self.Controllable` true)
      (`self.SetAnimationValues`)
      (`self.CalculateUIHealth`))))

(event `self.ReceiveTick`
  (params (DeltaSeconds :type "Float (single-precision)"))
  (bind _result (`self.CheckForDeath`))
  (if _result
    (if (`self.ForceStopMovement`)
      (`KismetSystemLibrary.Delay` 0.3)
      (set `self.ForceStopMovement` false))
    (if (`self.actuallyFired`)
      (`KismetSystemLibrary.Delay` 0.3)
      (set `self.actuallyFired` false))
    (if (`self.IsAttacking`)
      (`self.CheckAttack`)
      (elif (`self.IsInteracting`)
        (`self.CheckInteraction`)))
    (else
      (`/Engine/EditorBlueprintResources/StandardMacros.DoOnce` false
        (:`Completed`
          (`PrimitiveComponent.SetCollisionResponseToAllChannels` (`self.CapsuleComponent`) "ECR_Ignore")
          ;[1 1 1] Deletion zone
          (`Controller.UnPossess` (`self.GetController`))
          (`SceneComponent.K2_SetWorldLocation` (`self.MinimapIcon`) (0.0 0.0 -200.0) false true)
          (`KismetSystemLibrary.Delay` 2.0)
          (`self.PlayerDead` (`self.Panel index`))
          (`self.K2_DestroyActor`))))))

(event `FireAtEnemy`
  (`/Engine/EditorBlueprintResources/StandardMacros.DoOnce` false
    (:`Completed`
      (`self.AttackTheEnemy`)
      (`KismetSystemLibrary.K2_SetTimer` null "AttackTheEnemy" (`self.AttackSpeed`) true))))

(event `EnemyHearingWithDelay`
  (`KismetSystemLibrary.Delay` (`KismetMathLibrary.RandomFloatInRange` 0.2 0.6))
  (bind _outactors (`GameplayStatics.GetAllActorsOfClass` "/Game/Enemy/BP_EnemyCharacter.BP_EnemyCharacter_C"))
  (for _array_element _outactors
    (if (<= (`KismetMathLibrary.VSize` (- (`self.K2_GetActorLocation` _array_element) (`self.K2_GetActorLocation`))) (`self.HearingRadius`))
      (bind _returnvalue (`AIBlueprintHelperLibrary.GetBlackboard` (`AIBlueprintHelperLibrary.GetAIController` _array_element)))
      (if (`KismetSystemLibrary.IsValid` _returnvalue)
        (`BlackboardComponent.SetValueAsObject` _returnvalue (`self.ActiveEnemyKey`) self)
        (`BlackboardComponent.SetValueAsEnum` _returnvalue (`self.fgntyjjtyj`) (`self.fergvjnegoentbrt`))
        (else
          (`KismetSystemLibrary.PrintString` "bb not valid"))))))

(fn `AddWeapon`
  (params (WeaponPosition :type "Vector Structure") (Weapon :type "/Game/Gameplay/Combat/Weapon Class Reference"))
  (bind _character_weapon (`self.Character weapon`))
  (bind _mesh (`self.Mesh`))
  (bind _returnvalue (`|SpawnActorFromClass` Weapon (`SceneComponent.K2_GetComponentToWorld` _mesh) "Undefined" "OverrideRootScale"))
  (bind _output_get (set `self.Character weapon` _returnvalue))
  (`SceneComponent.K2_AttachToComponent` (`/Game/Gameplay/Combat/Weapon.DefaultSceneRoot` _output_get) _mesh "GunSocket" "SnapToTarget" "SnapToTarget" "KeepWorld" true)
  (set `self.CanAttack` true)
  (set `self.WeaponRadius` 500.0)
  (if (== Weapon "/Game/Gameplay/Combat/Weapon.Weapon_C")
    (`SkeletalMeshComponent.SetAnimInstanceClass` (`self.Mesh`) "/Game/AnimStarterPack/AnimBlueprintRifle.AnimBlueprintRifle_C")
    (set `self.CharacterIcon` "/Game/Textures2D/gun_icon.gun_icon")
    (else
      (`SkeletalMeshComponent.SetAnimInstanceClass` (`self.Mesh`) "/Game/AnimStarterPack/AnimBlueprintShotgun.AnimBlueprintShotgun_C")
      (set `self.CharacterIcon` "/Game/Textures2D/hunting_shotgun.hunting_shotgun")))
  (`self.K2_SetActorRotation` (`KismetMathLibrary.MakeRotator` 0.0 0.0 (.yaw (`KismetMathLibrary.FindLookAtRotation` (`self.K2_GetActorLocation`) (`local.WeaponPosition`)))))
  (`self.SetAnimationValues`)
  (`ActorComponent.Activate` (`self.PickupSound`) false)
  (set `self.WeaponRadius` (`/Game/Gameplay/Combat/Weapon.WeaponRadius` _character_weapon))
  (set `self.AttackSpeed` (`/Game/Gameplay/Combat/Weapon.WeaponAttackSpeed` _character_weapon)))

(fn `AttackTheEnemy`
  (bind _capsulecomponent (`self.CapsuleComponent`))
  (`|ExecutionSequence`
    (:`then_1`
      (if (`KismetSystemLibrary.IsValid` (`self.EnemyTarget`))
        (set `/Game/Gameplay/Combat/Weapon.Target` (`self.EnemyTarget`) (`self.Character weapon`))
        (`|ExecutionSequence`
          (:`then_0`
            (`self.EnemyHearingWithDelay`))
          (:`then_1`
            (if (`self.IsAttacking`)
              (`/Game/Gameplay/Combat/Weapon.Fire` (`self.Character weapon`))
              (`/Engine/EditorBlueprintResources/StandardMacros.DoOnce` false
                (:`Completed`
                  (set `self.actuallyFired` true)
                  (`SceneComponent.K2_SetWorldRotation` _capsulecomponent (`KismetMathLibrary.MakeRotator` (.roll (`SceneComponent.K2_GetComponentRotation` _capsulecomponent)) 0.0 (.yaw (`SceneComponent.K2_GetComponentRotation` _capsulecomponent))) false false))))))
        (else
          (set `self.IsAttacking` false))))))

(fn `CalculateUIHealth`
  (set `self.CharacterHealth_0` (/ (`self.CharacterHealth`) 100.0))
  (if (< (`self.CharacterHealth`) 0.0)
    (set `self.IsDead` true)))

(fn `CheckAttack`
  (bind _result (`self.CheckForDeath`))
  (if _result
    (if (`KismetSystemLibrary.IsValid` (`self.EnemyTarget`))
      (bind _asgit_character (cast `GitCharacter` (`self.EnemyTarget`)))
      (if (`GitCharacter.IsDead` _asgit_character)
        (set `self.IsAttacking` false :!label _label)
        (`MovementComponent.StopMovementImmediately` (`self.CharacterMovement`))
        (else
          (`self.FollowEnemyIfNeeded`)
          (if (`self.CanAttack`)
            (if (`self.AbleToFire`)
              (`self.AttackTheEnemy`)
              (`NavMovementComponent.StopActiveMovement` (`self.CharacterMovement`))
              (set `self.ForceStopMovement` true)
              (else
                (`self.CheckRayPosition`)))
            (else
              (goto _label)))))
      (else
        (goto _label)))
    (else
      (set `self.IsAttacking` false))))

(fn `CheckDistance`
  (if (<= (`self.GetDistanceTo` (`self.EnemyTarget`)) (`self.WeaponRadius`))
    (set `self.AbleToFire` true)
    (`NavMovementComponent.StopActiveMovement` (`self.CharacterMovement`))
    (bind _asbp_enemy_character (cast `/Game/Enemy/BP_EnemyCharacter` (`self.EnemyTarget`)))
    (`SceneComponent.K2_SetWorldRotation` (`self.CapsuleComponent`) (`KismetMathLibrary.FindLookAtRotation` (`SceneComponent.K2_GetComponentLocation` (`self.Weapon Pos`)) (`SceneComponent.K2_GetComponentLocation` (`/Game/Enemy/BP_EnemyCharacter.Hitbox` _asbp_enemy_character))) false false)
    (elif (`self.AbleToFire`)
      (set `self.AbleToFire` false))))

(fn `CheckDistanceAtItem`
  (params (Target :type "Actor Object Reference"))
  (returns (Result :type Boolean))
  (return (<= (`self.GetDistanceTo` Target) (`self.LootRadius`))))

(fn `CheckForDeath`
  (returns (Result :type Boolean))
  (if (`self.IsDead`)
    (set `self.IsAttacking` false)
    (return false)
    (else
      (return true))))

(fn `CheckInteraction`
  (bind _targetitem (`self.TargetItem`))
  (if (`KismetSystemLibrary.IsValid` (`self.TargetItem`))
    (bind _result (`self.CheckRayPositionAtItem` _targetitem))
    (if _result
      (bind _result_2 (`self.CheckDistanceAtItem` _targetitem))
      (if _result_2
        (`self.StopMovementAtItem` _targetitem)
        (set `self.IsInteracting` false)
        (bind _aspickable_game_item (cast `/Game/Player/PickableGameItem` (`self.TargetItem`)))
        (message `/Game/Gameplay/Combat/iInteractableItem.Init interaction` _aspickable_game_item self)))
    (else
      (set `self.IsInteracting` false)
      (`MovementComponent.StopMovementImmediately` (`self.CharacterMovement`)))))

(fn `CheckPickup`)

(fn `CheckRayPosition`
  (bind _outhit (`KismetSystemLibrary.LineTraceSingle` (`self.K2_GetActorLocation` (`self.EnemyTarget`)) (`SceneComponent.K2_GetComponentLocation` (`self.Hitbox`)) "TraceTypeQuery3"))
  (if (not (`GameplayStatics.BreakHitResult` _outhit))
    (`self.CheckDistance`)))

(fn `CheckRayPositionAtItem`
  (params (Target :type "Actor Object Reference"))
  (returns (Result :type Boolean))
  (bind _outhit (`KismetSystemLibrary.LineTraceSingle` (`self.K2_GetActorLocation` Target) (`SceneComponent.K2_GetComponentLocation` (`self.Hitbox`)) "TraceTypeQuery3"))
  (if (`GameplayStatics.BreakHitResult` _outhit)
    (return false)
    (else
      (return true))))

(fn `DisableSelectionRing`
  (bind _minimapicon (`self.MinimapIcon`))
  (`SceneComponent.SetVisibility` (`self.Selection ring decal`) false false)
  (`/Engine/EditorBlueprintResources/StandardMacros.IsValid` _minimapicon
    (:`Is Valid`
      (`PaperSpriteComponent.SetSpriteColor` _minimapicon (struct :`R` 1.0 :`G` 1.0 :`A` 1.0)))))

(fn `EnableSelectionRing`
  (`SceneComponent.SetVisibility` (`self.Selection ring decal`) true false)
  (`PaperSpriteComponent.SetSpriteColor` (`self.MinimapIcon`) (struct :`R` 0.055961 :`G` 0.495 :`B` 0.081597 :`A` 1.0)))

(fn `FollowEnemyIfNeeded`
  (if (not (`self.ForceStopMovement`))
    (`self.CheckRayPosition`)
    (if (not (`self.AbleToFire`))
      (`NavigationSystem.SimpleMoveToLocation` (`self.GetController`) (`self.K2_GetActorLocation` (`self.EnemyTarget`))))))

(fn `IsCloseEnough`
  (returns (Result :type Boolean))
  (bind _result (`self.CheckRayPositionAtItem` (`self.EnemyTarget`)))
  (if _result
    (bind _result_2 (`self.CheckDistanceAtItem` (`self.EnemyTarget`)))
    (if _result_2
      (return true)
      (else
        (return false)))
    (else
      (return false))))

(fn `IsValidTarget`
  (params (`Spawn point` :type "Vector Structure"))
  (returns (Result :type Boolean))
  (return (>= (`KismetMathLibrary.VSize` (- (`self.K2_GetActorLocation`) `Spawn point`)) 60.0)))

(fn `SetAnimationValues`
  (bind _animclass (`SkeletalMeshComponent.AnimClass` (`self.Mesh`)))
  (if (`self.CanAttack`)
    (castclass `/Game/AnimStarterPack/UE4ASP_HeroTPP_AnimBlueprint` _animclass)
    (else
      (castclass `/Game/AnimStarterPack/NoGunCharacterAnimation` _animclass))))

(fn `StopMovementAtItem`
  (params (Target :type "Actor Object Reference"))
  (`NavMovementComponent.StopActiveMovement` (`self.CharacterMovement`))
  (`SceneComponent.K2_SetWorldRotation` (`self.CapsuleComponent`) (`KismetMathLibrary.FindLookAtRotation` (`self.K2_GetActorLocation`) (`self.K2_GetActorLocation` Target)) false false))

(fn `UserConstructionScript`)