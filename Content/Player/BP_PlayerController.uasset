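; Player controller Blueprint holding an unfinished or disabled mouse-to-world targeting trace.
; The EventGraph logic has no event driving it, so it never runs, and the construction script is empty.
; As written, it traces on Visibility from CameraRef's location along the deprojected cursor direction, ignoring CameraRef, and stores the hit location in TargetDestination.
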(fn `UserConstructionScript`)