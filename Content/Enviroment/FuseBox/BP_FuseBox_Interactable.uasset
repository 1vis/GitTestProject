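; Interactable fuse box that, on its first interaction, sends a power outage message to every IPowerable actor and reveals its particle effect.
; Cursor hover toggles a decal ring and UI panel, both hidden at BeginPlay along with the particles.
; While the panel is visible, Tick rotates its scene component to follow the main arm of the player controller's active BP_Camera, cached at BeginPlay.
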(event `/Game/Gameplay/Combat/iInteractableItem.Init interaction`
  (params (`Actor that interacts with this item` :type "Actor Object Reference"))
  ;[1 1 1] Tato funkcia sa vola ked je character dostatocne blizko n interakciu
  (`/Engine/EditorBlueprintResources/StandardMacros.DoOnce` false
    (:`Completed`
      (bind _outactors (`GameplayStatics.GetAllActorsWithInterface` "/Game/AAAAAA/IPowerable.IPowerable_C"))
      (for _array_element _outactors
        (message `/Game/AAAAAA/IPowerable.OnPowerOutage` _array_element)
        (`SceneComponent.SetVisibility` (`self.ParticleSystem`) true false)))))

(event `self.ReceiveBeginPlay`
  (`|ExecutionSequence`
    (:`then_0`
      (`SceneComponent.SetVisibility` (`self.ParticleSystem`) false false))
    (:`then_1`
      (`self.Init`)
      (bind _asbp_git_player_controller (cast `/Game/Player/BP_GitPlayerController` (`GameplayStatics.GetPlayerController` 0)))
      (bind _asbp_camera (cast `/Game/Player/BP_Camera` (`GitPlayerController.ActiveCamera` _asbp_git_player_controller)))
      (set `self.WorldCamera` _asbp_camera)
      (add `self.OnBeginCursorOver` (delegate `CustomEvent`))
      (add `self.OnEndCursorOver` (delegate `CustomEvent_1`)))))

(event `self.ReceiveTick`
  (params (DeltaSeconds :type "Float (single-precision)"))
  (`self.RotateUIPanelCorrectly`))

(event `CustomEvent_1` :!signature `self.OnEndCursorOver`
  (params (TouchedActor :type "Actor Object Reference"))
  ;[1 1 1] Hide visibillity ring
  (`SceneComponent.SetVisibility` (`self.Decal`) false false)
  (`SceneComponent.SetVisibility` (`self.Panel`) false false))

(event `CustomEvent` :!signature `self.OnBeginCursorOver`
  (params (TouchedActor :type "Actor Object Reference"))
  ;[1 1 1] Show visibillity ring
  (`SceneComponent.SetVisibility` (`self.Decal`) true false)
  (`SceneComponent.SetVisibility` (`self.Panel`) true false))

(fn `Init`
  (`SceneComponent.SetVisibility` (`self.Decal`) false false)
  (`SceneComponent.SetVisibility` (`self.Panel`) false false))

(fn `RotateUIPanelCorrectly`
  (if (`SceneComponent.IsVisible` (`self.Panel`))
    (`SceneComponent.K2_SetWorldRotation` (`self.Scene`) (`KismetMathLibrary.MakeRotator` (.roll (`SceneComponent.K2_GetComponentRotation` (`/Game/Player/BP_Camera.MainArm` (`self.WorldCamera`)))) (- 90.0 (* (.pitch (`SceneComponent.K2_GetComponentRotation` (`/Game/Player/BP_Camera.MainArm` (`self.WorldCamera`)))) -1.0)) (.yaw (`SceneComponent.K2_GetComponentRotation` (`/Game/Player/BP_Camera.MainArm` (`self.WorldCamera`))))) false false)))

(fn `UserConstructionScript`
  (`parent.UserConstructionScript`))