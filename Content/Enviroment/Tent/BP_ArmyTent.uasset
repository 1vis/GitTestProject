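; Army tent environment actor with a lit doorway and windows that go dark during a power outage.
; The construction script toggles between the closed door and the door light based on a closed-door setting.
; OnPowerOutage hides the door light and sets the MainColor material parameter on the door and each window to the black color.
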(event `self.ReceiveBeginPlay`)

(event `/Game/AAAAAA/IPowerable.OnPowerOutage`
  (`SceneComponent.SetHiddenInGame` (`self.DoorLight`) true false)
  (`MeshComponent.SetVectorParameterValueOnMaterials` (`self.Door`) "MainColor" (`KismetMathLibrary.Conv_LinearColorToVector` (`self.BlackColor`)))
  (`MeshComponent.SetVectorParameterValueOnMaterials` (`self.Window`) "MainColor" (`KismetMathLibrary.Conv_LinearColorToVector` (`self.BlackColor`)))
  (`MeshComponent.SetVectorParameterValueOnMaterials` (`self.Window2`) "MainColor" (`KismetMathLibrary.Conv_LinearColorToVector` (`self.BlackColor`)))
  (`MeshComponent.SetVectorParameterValueOnMaterials` (`self.Window3`) "MainColor" (`KismetMathLibrary.Conv_LinearColorToVector` (`self.BlackColor`)))
  (`MeshComponent.SetVectorParameterValueOnMaterials` (`self.Window4`) "MainColor" (`KismetMathLibrary.Conv_LinearColorToVector` (`self.BlackColor`)))
  (`MeshComponent.SetVectorParameterValueOnMaterials` (`self.Window5`) "MainColor" (`KismetMathLibrary.Conv_LinearColorToVector` (`self.BlackColor`)))
  (`MeshComponent.SetVectorParameterValueOnMaterials` (`self.WIndow6`) "MainColor" (`KismetMathLibrary.Conv_LinearColorToVector` (`self.BlackColor`)))
  (`MeshComponent.SetVectorParameterValueOnMaterials` (`self.Window7`) "MainColor" (`KismetMathLibrary.Conv_LinearColorToVector` (`self.BlackColor`)))
  (`MeshComponent.SetVectorParameterValueOnMaterials` (`self.Window8`) "MainColor" (`KismetMathLibrary.Conv_LinearColorToVector` (`self.BlackColor`))))

(fn `UserConstructionScript`
  (bind _closeddoor (`self.ClosedDoor`))
  (bind _doorlight (`self.DoorLight`))
  (if (`self.ClosedDoor?`)
    (`SceneComponent.SetVisibility` _closeddoor true false)
    (`SceneComponent.SetVisibility` _doorlight false false)
    (else
      (`SceneComponent.SetVisibility` _closeddoor false false)
      (`SceneComponent.SetVisibility` _doorlight true false))))